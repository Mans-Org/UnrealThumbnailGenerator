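; Sky sphere actor that displays the environment cubemap as the backdrop of a thumbnail generator scene.
; The construction script creates a dynamic instance of the thumbnail sky material on the sphere mesh.
; On each scene update it blocking-loads the cubemap from the settings, shows the sphere only if that loads and the environment is enabled, then applies its tint, rotation and texture to the material.
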(event `ThumbnailSceneInterface.OnUpdateThumbnailScene`
  (params (ThumbnailSettings :type "ThumbnailSettings Structure (by ref)"))
  (bind ((`bShowEnvironment` _bshowenvironment) (`EnvironmentColor` _environmentcolor) (`EnvironmentCubeMap` _environmentcubemap) (`EnvironmentRotation` _environmentrotation)) (break `ThumbnailSettings` ThumbnailSettings))
  (bind _returnvalue (`KismetSystemLibrary.LoadAsset_Blocking` _environmentcubemap))
  (bind _returnvalue_2 (and (`KismetSystemLibrary.IsValid` _returnvalue) _bshowenvironment))
  (`SceneComponent.SetVisibility` (`self.SkySphereMesh`) _returnvalue_2 false)
  (if _returnvalue_2
    (`MaterialInstanceDynamic.SetVectorParameterValue` (`self.Sky material`) "Tint" _environmentcolor)
    (`MaterialInstanceDynamic.SetScalarParameterValue` (`self.Sky material`) "CubemapRotation" _environmentrotation)
    (`MaterialInstanceDynamic.SetTextureParameterValue` (`self.Sky material`) "Skybox" (cast `Texture` _returnvalue :!pure true))))

(fn `UserConstructionScript`
  (bind _returnvalue (`PrimitiveComponent.CreateDynamicMaterialInstance` (`self.SkySphereMesh`) 0 "/ThumbnailGenerator/SkySphere/M_ThumbnailGenerator_Sky.M_ThumbnailGenerator_Sky" "None"))
  (set `self.Sky material` _returnvalue))